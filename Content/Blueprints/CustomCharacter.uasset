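; Player character Blueprint with movement, camera look, jump, Shift sprint, a ranged attack and death handling.
; Axis inputs drive yaw-relative movement, while Q spawns a Projectile at the ControlCamera position with actor rotation and plays a roar montage.
; AnyDamage sets Health to Damage minus Health, reversing the usual subtraction, and a positive check spawns a death effect and destroys the actor.
; A separate DeathEvent graph duplicates that death sequence.
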(event `Key|LeftShift`
  (params (Key :type "Key Structure" :default "AnyKey"))
  ;[1 1 1] 달리기
  (:`Pressed`
    (set `CharacterMovementComponent.MaxWalkSpeed` 900.0 (`self.CharacterMovement`)))
  (:`Released`
    (set `CharacterMovementComponent.MaxWalkSpeed` 270.0 (`self.CharacterMovement`))))

(event `self.ReceiveAnyDamage`
  (params (Damage :type "Float (single-precision)") (DamageType :type "DamageType Object Reference") (InstigatedBy :type "Controller Object Reference") (DamageCauser :type "Actor Object Reference"))
  (bind _returnvalue (- Damage (`self.Health`)))
  ;[1 1 1] Death
  (set `self.Health` _returnvalue)
  (if (> _returnvalue 0.0)
    (`GameplayStatics.SpawnEmitterAtLocation` (`self.DeathEffect`) (`self.K2_GetActorLocation`))
    (`self.K2_DestroyActor`)))

(event `Key|Q`
  (params (Key :type "Key Structure" :default "AnyKey"))
  (:`Pressed`
    (`|SpawnActorFromClass` (`self.Projectile`) (`KismetMathLibrary.MakeTransform` (`SceneComponent.GetSocketLocation` (`self.ControlCamera`) "None") (`self.K2_GetActorRotation`)) "Undefined" "OverrideRootScale")
    (`AnimInstance.Montage_Play` (`SkeletalMeshComponent.GetAnimInstance` (`self.Mesh`)) "/Game/LowPolySkeleton/Skeleton_Grunt/Anims/roar_montage.roar_montage" 1.0)))

(event `InputAxis|Turn`
  (params (AxisValue :type "Float (single-precision)"))
  ;[1 1 1] 플레이어 카메라 동작
  (`self.AddControllerYawInput` AxisValue))

(event `InputAction|Jump`
  (params (Key :type "Key Structure" :default "AnyKey"))
  ;[1 1 1] 점프
  (:`Pressed`
    (`self.Jump`)))

(event `InputAxis|LookUp`
  (params (AxisValue :type "Float (single-precision)"))
  ;[1 1 1] 플레이어 카메라 동작
  (`self.AddControllerPitchInput` AxisValue))

(event `InputAxis|MoveForward`
  (params (AxisValue :type "Float (single-precision)"))
  ;[1 1 1] 이동구현
  (`self.AddMovementInput` (`KismetMathLibrary.GetForwardVector` (`KismetMathLibrary.MakeRotator` 0.0 0.0 (.yaw (`self.K2_GetActorRotation`)))) AxisValue))

(event `InputAxis|MoveRight`
  (params (AxisValue :type "Float (single-precision)"))
  ;[1 1 1] 이동구현
  (`self.AddMovementInput` (`KismetMathLibrary.GetRightVector` (`KismetMathLibrary.MakeRotator` 0.0 0.0 (.yaw (`self.K2_GetActorRotation`)))) AxisValue))

(fn `DeathEvent`
  (`GameplayStatics.SpawnEmitterAtLocation` (`self.DeathEffect`) (`self.K2_GetActorLocation`))
  (`self.K2_DestroyActor`))

(fn `UserConstructionScript`)